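; Openable door actor that swings open and closed through OpenDoor's OnOpen and OnClose events.
; The DoorState timeline plays on open and reverses on close, applying its OpenAngle track as a yaw offset combined with the rotation cached at BeginPlay.
; An event track on the same timeline plays a steam sound cue at the door's location.
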(event `self.ReceiveBeginPlay`
  (set `self.Intial Rotation` (`self.K2_GetActorRotation`)))

(event `self.OpenDoor.OnOpen`
  (bind (_direction _open_angle) (`Timeline|Door state` :!label _label)
    (:`Update`
      (`self.K2_SetActorRotation` (`KismetMathLibrary.ComposeRotators` (`KismetMathLibrary.MakeRotator` 0.0 0.0 _open_angle) (`self.Intial Rotation`))))
    (:`SonudTimming`
      (`GameplayStatics.PlaySoundAtLocation` "/Game/StarterContent/Audio/Steam01_Cue.Steam01_Cue" (`self.K2_GetActorLocation`) (struct) 1.0 1.0 0.0 null null null))))

(event `self.OpenDoor.OnClose`
  (goto _label :!via `Reverse`))

(fn `UserConstructionScript`)